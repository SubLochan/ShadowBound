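; Enemy AI character that roams randomly, chases any pawn it sees and punches it on arrival.
; An enum-driven UpdateBrain event switches between idle, roam, chase and death, adjusting walk speed and using AI MoveTo.
; Punches signal the Anim Instance by message; a dead target disables sensing and resumes roaming.
; Damage updates an HP bar, shown while the player overlaps a sphere, and death destroys the actor after a delay.
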(event `self.PawnSensing.OnSeePawn`
  (params (Pawn :type "Pawn Object Reference"))
  (set `self.Player` Pawn)
  (`self.Update Brain` "NewEnumerator1"))

(event `self.ReceiveBeginPlay`
  (`self.f_AIWidgetHP`)
  (`self.Update Brain` "NewEnumerator0")
  (`PawnSensingComponent.SetPeripheralVisionAngle` (`self.PawnSensing`) 180.0))

(event `self.Sphere.OnComponentBeginOverlap`
  (params (OverlappedComponent :type "PrimitiveComponent Object Reference") (OtherActor :type "Actor Object Reference") (OtherComp :type "PrimitiveComponent Object Reference") (OtherBodyIndex :type Integer) (bFromSweep :type Boolean) (SweepResult :type "HitResult Structure (by ref)"))
  (cast `/Game/Blueprints/CharacterBP/BP_ThirdPersonCharacter` OtherActor)
  (`SceneComponent.SetHiddenInGame` (`self.Widget`) false false))

(event `Update Brain`
  (params (`AI Brain` :type "/Game/Blueprints/AI_Characters/Enum_AI_Brain Enum" :default "NewEnumerator2"))
  (bind _returnvalue (`SkeletalMeshComponent.GetAnimInstance` (`self.Mesh`)))
  (if (`self.Is AI Alive?`)
    (switch `/Game/Blueprints/AI_Characters/Enum_AI_Brain` `AI Brain`
      (:`NewEnumerator2`
        (`self.f_setAI_MaxSpeed` 150.0))
      (:`NewEnumerator0`
        (`self.f_setAI_MaxSpeed` 150.0)
        (`self.AI Random Roam`))
      (:`NewEnumerator1`
        (`self.f_setAI_MaxSpeed` 450.0)
        (`|AIMoveTo` self (0.0 0.0 0.0) (`self.Player`) 100.0
          (:`OnSuccess`
            (bind _is_alive__ (`self.f_IsPlayerAlive?`))
            (if _is_alive__
              (message `/Game/Blueprints/AI_Characters/AI_IF.Enum_AI` _returnvalue true)
              (`KismetSystemLibrary.Delay` 0.5)
              (message `/Game/Blueprints/AI_Characters/AI_IF.Enum_AI` _returnvalue false)
              (else
                (`PawnSensingComponent.SetSensingUpdatesEnabled` (`self.PawnSensing`) false)
                (`KismetSystemLibrary.Delay` 3.0)
                (`self.Update Brain` "NewEnumerator0"))))
          (:`OnFail`
            (`self.Update Brain` "NewEnumerator0"))))
      (:`NewEnumerator3`
        (`CharacterMovementComponent.SetMovementMode` (`self.CharacterMovement`) "MOVE_None" 0)
        (set `self.Is AI Alive?` false)))))

(event `self.Sphere.OnComponentEndOverlap`
  (params (OverlappedComponent :type "PrimitiveComponent Object Reference") (OtherActor :type "Actor Object Reference") (OtherComp :type "PrimitiveComponent Object Reference") (OtherBodyIndex :type Integer))
  (cast `/Game/Blueprints/CharacterBP/BP_ThirdPersonCharacter` OtherActor)
  (`SceneComponent.SetHiddenInGame` (`self.Widget`) true false))

(event `self.ReceiveAnyDamage`
  (params (Damage :type "Float (single-precision)") (DamageType :type "DamageType Object Reference") (InstigatedBy :type "Controller Object Reference") (DamageCauser :type "Actor Object Reference"))
  (if (>= (`self.HP`) 0.0)
    (set `self.HP` (- (`self.HP`) Damage))
    (`self.f_AIWidgetHP`)
    ;[0 0 0] On Death
    (`self.PlayAnimMontage` "/Game/AI/Frog/CharacterArmature_HitReact_Montage.CharacterArmature_HitReact_Montage")
    (if (<= (`self.HP`) 0.0)
      (`SkeletalMeshComponent.PlayAnimation` (`self.Mesh`) "/Game/AI/Frog/CharacterArmature_Death.CharacterArmature_Death" false)
      (`ActorComponent.K2_DestroyComponent` (`self.PawnSensing`))
      (`ActorComponent.K2_DestroyComponent` (`self.Sphere`))
      (`SceneComponent.SetHiddenInGame` (`self.Widget`) true false)
      (`self.Update Brain` "NewEnumerator3")
      (`KismetSystemLibrary.Delay` 15.0)
      (`self.K2_DestroyActor`))))

(fn `f_AIWidgetHP`
  (bind _asai_hp (cast `/Game/Blueprints/AI_Characters/AI_HP` (`WidgetComponent.GetWidget` (`self.Widget`))))
  (`ProgressBar.SetPercent` (`/Game/Blueprints/AI_Characters/AI_HP.ProgressBar_HP` _asai_hp) (/ (`self.HP`) 100.0)))

(fn `f_IsPlayerAlive?`
  (returns (`Is Alive ?` :type Boolean))
  (bind _is_alive__ (message `/Game/Blueprints/AI_Characters/AI_IF.Is Player Alive?` (`self.Player`)))
  (return _is_alive__))

(fn `f_setAI_MaxSpeed`
  (params (`Max Walk Speed` :type "Float (single-precision)"))
  (set `CharacterMovementComponent.MaxWalkSpeed` `Max Walk Speed` (`self.CharacterMovement`)))

(fn `UserConstructionScript`)