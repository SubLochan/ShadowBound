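; POI_Component marks its owning actor as a point of interest for the map system.
; One second after BeginPlay, it finds the BP_MapSystem actor and, if valid, adds its owner to that actor's POIActors list.
; When ShowOnMinimap is set, it also asks the map system to show the owner on the minimap, passing its image, size and static flag.
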(event `self.ReceiveBeginPlay`
  (`KismetSystemLibrary.Delay` 1.0)
  (bind _returnvalue (`GameplayStatics.GetActorOfClass` "/Game/Blueprints/MapSystem/BP_MapSystem.BP_MapSystem_C"))
  (`/Engine/EditorBlueprintResources/StandardMacros.IsValid` _returnvalue
    (:`Is Valid`
      (`KismetArrayLibrary.Array_Add` (`/Game/Blueprints/MapSystem/BP_MapSystem.POI_Actors` _returnvalue) (`self.GetOwner`))
      (if (`self.Show On Minimap ?`)
        (`/Game/Blueprints/MapSystem/BP_MapSystem.Show POI On Minimap` _returnvalue (`self.POI Image`) (`self.GetOwner`) (`self.Is Static ?`) (`self.POI Size`))))))