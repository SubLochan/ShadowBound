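; Map manager that puts a minimap on screen and toggles a full map via the M key or OpenMap.
; BeginPlay creates the minimap; each map opening builds a fresh widget with icons for POIActors, using AC_POI_Component images and removing invalid actors mid-loop.
; ShowPOIOnMinimap adds icons to the minimap overlay on request, and HideMap sets minimap visibility.
; Level dimensions and minimap zoom are passed into the widgets.
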(event `self.ReceiveBeginPlay`
  (`self.EnableInput` (`GameplayStatics.GetPlayerController` 0))
  (bind _returnvalue (`|CreateWidget` "/Game/Blueprints/MapSystem/MiniMap/WBP_MiniMap.WBP_Minimap_C" null (`self.Level Dimension`) (`self.Mini Map Zoom`) (`self.Map Texture`)))
  (bind _output_get (set `self.Minimap` _returnvalue))
  (`UserWidget.AddToViewport` _output_get 0))

(event `Open Map`
  (`/Engine/EditorBlueprintResources/StandardMacros.FlipFlop` :!label _label
    (:`A`
      (bind _returnvalue (`|CreateWidget` "/Game/Blueprints/MapSystem/WBP_MainMap.WBP_MainMap_C" null (`self.Level Dimension`)))
      (`Image.SetBrushFromTexture` (`/Game/Blueprints/MapSystem/WBP_MainMap.Map_Image` _returnvalue) (`self.Map Texture`) false)
      (`UserWidget.AddToViewport` _returnvalue 0)
      (for _array_element (`self.POI_Actors`)
        (`/Engine/EditorBlueprintResources/StandardMacros.IsValid` _array_element
          (:`Is Valid`
            (bind _returnvalue_2 (`|CreateWidget` "/Game/Blueprints/MapSystem/WBP_POI.WBP_POI_C" null (`/Game/Blueprints/BlueprintComponents/AC_POI_Component.POI Image` (`self.GetComponentByClass` _array_element "/Game/Blueprints/BlueprintComponents/AC_POI_Component.AC_POI_Component_C")) _array_element (`self.Level Dimension`) (`self.Canvas Dimension`)))
            (bind _returnvalue_3 (`Overlay.AddChildToOverlay` (`/Game/Blueprints/MapSystem/WBP_MainMap.Overlay_MainMap` _returnvalue) _returnvalue_2))
            (`OverlaySlot.SetHorizontalAlignment` _returnvalue_3 "HAlign_Center")
            (`OverlaySlot.SetVerticalAlignment` _returnvalue_3 "VAlign_Center"))
          (:`Is Not Valid`
            (`KismetArrayLibrary.Array_RemoveItem` (`self.POI_Actors`) _array_element)))))
    (:`B`
      (`Widget.RemoveFromParent` _returnvalue))))

(event `Key|M`
  (params (Key :type "Key Structure"))
  (:`Pressed`
    (goto _label)))

(event `Show POI On Minimap`
  (params (`POI Image` :type "Texture2D Object Reference") (`POI Owner Actor` :type "Actor Object Reference") (`Is Static ?` :type Boolean) (POI_Size :type "Float (double-precision)"))
  (bind _returnvalue (`|CreateWidget` "/Game/Blueprints/MapSystem/WBP_POI_Minimap.WBP_POI_Minimap_C" null `POI Image` `POI Owner Actor` (`self.Level Dimension`) (`self.Minmap Dimension`) (`self.Mini Map Zoom`) POI_Size))
  (bind _returnvalue_2 (`Overlay.AddChildToOverlay` (`/Game/Blueprints/MapSystem/MiniMap/WBP_MiniMap.Overlay_Minimap` (`self.Minimap`)) _returnvalue))
  (`OverlaySlot.SetHorizontalAlignment` _returnvalue_2 "HAlign_Center")
  (`OverlaySlot.SetVerticalAlignment` _returnvalue_2 "VAlign_Center"))

(event `Hide Map`
  (params (`Hide Minimap UI ?` :type Boolean))
  (bind _minimap (`self.Minimap`))
  (if `Hide Minimap UI ?`
    (set `Widget.Visibility` "Hidden" _minimap)
    (else
      (set `Widget.Visibility` "SelfHitTestInvisible" _minimap))))

(fn `UserConstructionScript`)