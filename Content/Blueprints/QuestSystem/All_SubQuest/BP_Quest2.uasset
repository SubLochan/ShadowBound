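; BP_Quest2 is a sub-quest Blueprint in the quest system that tracks an item-collection objective through its Mushroom event.
; The event adds the passed amount to the QuestSystem have count and rebuilds the need/have progress text.
; It then calls UpdateQuestUI on WBP_Quest_Book, fetched with GetActorOfClass, and prints whether the needed count is reached, with no further completion handling.
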(event `/Game/Blueprints/QuestSystem/IF_Quest.Mushroom`
  (params (Mushroom :type Integer))
  (bind _questsystem (`self.QuestSystem`))
  (bind _questsystem_2 (`self.QuestSystem`))
  (bind _output_get (set `/Game/Blueprints/QuestSystem/QuestSystem.Have Item` (+ Mushroom (`/Game/Blueprints/QuestSystem/QuestSystem.Have Item` _questsystem)) _questsystem))
  (set `/Game/Blueprints/QuestSystem/QuestSystem.Quest Items` (`|FormatText` "Item {Need} / {Have}" (`/Game/Blueprints/QuestSystem/QuestSystem.Need Item` _questsystem) _output_get) (`self.QuestSystem`))
  (bind _returnvalue (`GameplayStatics.GetActorOfClass` "/Game/Blueprints/QuestSystem/QuestBook/WBP_Quest_Book.WBP_Quest_Book_C"))
  (`/Game/Blueprints/QuestSystem/QuestBook/WBP_Quest_Book.Update Quest UI` _returnvalue)
  (`KismetSystemLibrary.PrintString` (`KismetStringLibrary.Conv_BoolToString` (>= (`/Game/Blueprints/QuestSystem/QuestSystem.Have Item` _questsystem_2) (`/Game/Blueprints/QuestSystem/QuestSystem.Need Item` _questsystem_2)))))

(fn `UserConstructionScript`)