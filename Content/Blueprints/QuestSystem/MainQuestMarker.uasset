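; MainQuestMarker is a quest marker actor that displays the player's distance to it through a Marker widget.
; Every tick it measures the distance to the player character, converts it to whole hundreds of units (metres at default scale) and writes it to the widget's Distance text.
; Its static mesh's begin-overlap event casts the other actor to BP_ThirdPersonCharacter but takes no further action.
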(event `self.ReceiveTick`
  (params (DeltaSeconds :type "Float (single-precision)"))
  (bind _asmarker (cast `/Game/Blueprints/QuestSystem/Marker` (`WidgetComponent.GetWidget` (`self.Widget`))))
  (set `/Game/Blueprints/QuestSystem/Marker.Distance` (`KismetTextLibrary.Conv_IntToText` (/ (`KismetMathLibrary.FTrunc` (`KismetMathLibrary.Vector_Distance` (`self.K2_GetActorLocation`) (`self.K2_GetActorLocation` (`GameplayStatics.GetPlayerCharacter` 0)))) 100)) _asmarker))

(event `self.StaticMesh.OnComponentBeginOverlap`
  (params (OverlappedComponent :type "PrimitiveComponent Object Reference") (OtherActor :type "Actor Object Reference") (OtherComp :type "PrimitiveComponent Object Reference") (OtherBodyIndex :type Integer) (bFromSweep :type Boolean) (SweepResult :type "HitResult Structure (by ref)"))
  (cast `/Game/Blueprints/CharacterBP/BP_ThirdPersonCharacter` OtherActor))

(fn `UserConstructionScript`)