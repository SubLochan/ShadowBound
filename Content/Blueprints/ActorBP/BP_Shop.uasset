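; Shop actor that lets the player buy and sell items through a UI shown while they overlap its box.
; It builds buy and sell entries from Inventory_DataTable, always listing static items but hiding other stock the player owns.
; Purchase and sale events update the player's PlayerInventory coins and items, refresh the UI and save.
; ISShopKeeperOnShop toggles the shopkeeper mesh and the box's overlap events to open or close trading.
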(event `self.ReceiveBeginPlay`)

(event `self.Box.OnComponentBeginOverlap`
  (params (OverlappedComponent :type "PrimitiveComponent Object Reference") (OtherActor :type "Actor Object Reference") (OtherComp :type "PrimitiveComponent Object Reference") (OtherBodyIndex :type Integer) (bFromSweep :type Boolean) (SweepResult :type "HitResult Structure (by ref)"))
  (bind _asbp_third_person_character (cast `/Game/Blueprints/CharacterBP/BP_ThirdPersonCharacter` OtherActor))
  (set `self.As BP Third Person Character` _asbp_third_person_character)
  (bind _returnvalue (`|CreateWidget` "/Game/Blueprints/Shop/WB_Shop_System.WB_Shop_System_C"))
  (set `self.Shop UI` _returnvalue)
  (`UserWidget.AddToViewport` (`self.Shop UI`) 0)
  (`self.f_Update Coin On UI`)
  (`self.f_Update Items On Shop`)
  (`self.f_Update Selling Item On UI`))

(event `self.Box.OnComponentEndOverlap`
  (params (OverlappedComponent :type "PrimitiveComponent Object Reference") (OtherActor :type "Actor Object Reference") (OtherComp :type "PrimitiveComponent Object Reference") (OtherBodyIndex :type Integer))
  (cast `/Game/Blueprints/CharacterBP/BP_ThirdPersonCharacter` OtherActor)
  (set `self.As BP Third Person Character` null)
  (bind _shop_ui (`self.Shop UI`)
    (:`then`
      (`Widget.RemoveFromParent` _shop_ui))
    (:`else`)))

(event `On Purchase Items`
  (params (`Item Name` :type String) (`Item Price` :type Integer) (`Item Store Quantity` :type Integer))
  (bind _returnvalue (`KismetStringLibrary.Conv_StringToName` `Item Name`))
  (if (>= (`/Game/Blueprints/BlueprintComponents/AC_Player_inventory.Coins` (`/Game/Blueprints/CharacterBP/BP_ThirdPersonCharacter.Player_inventory` (`self.As BP Third Person Character`))) `Item Price`)
    (set `/Game/Blueprints/BlueprintComponents/AC_Player_inventory.Coins` (- (`/Game/Blueprints/BlueprintComponents/AC_Player_inventory.Coins` (`/Game/Blueprints/CharacterBP/BP_ThirdPersonCharacter.Player_inventory` (`self.As BP Third Person Character`))) `Item Price`) (`/Game/Blueprints/CharacterBP/BP_ThirdPersonCharacter.Player_inventory` (`self.As BP Third Person Character`)))
    (`self.f_Update Coin On UI`)
    (`KismetArrayLibrary.Array_RemoveItem` (`self.Shop Items`) _returnvalue)
    (`self.f_Add Items On Inventory` _returnvalue)
    (`self.f_Add Items Quantity` `Item Store Quantity` _returnvalue)
    (`self.f_Clear All Shop Items`)
    (`self.f_Update Items On Shop`)
    ;[0 0 0] Save Data
    (`/Game/Blueprints/BlueprintComponents/AC_Player_inventory.f_SaveInventoryData` (`/Game/Blueprints/CharacterBP/BP_ThirdPersonCharacter.Player_inventory` (`self.As BP Third Person Character`)))))

(event `On Selling Items`
  (params (`Item Name` :type String) (`Selling Price` :type Integer))
  (bind _returnvalue (`KismetStringLibrary.Conv_StringToName` `Item Name`))
  (bind _player_inventory (`/Game/Blueprints/CharacterBP/BP_ThirdPersonCharacter.Player_inventory` (`self.As BP Third Person Character`)))
  (bind _player_inventory_2 (`/Game/Blueprints/CharacterBP/BP_ThirdPersonCharacter.Player_inventory` (`self.As BP Third Person Character`)))
  (`KismetArrayLibrary.Array_RemoveItem` (`/Game/Blueprints/BlueprintComponents/AC_Player_inventory.Items` _player_inventory) _returnvalue)
  (`BlueprintMapLibrary.Map_Remove` (`/Game/Blueprints/BlueprintComponents/AC_Player_inventory.Items Quantity` _player_inventory) _returnvalue)
  (set `/Game/Blueprints/BlueprintComponents/AC_Player_inventory.Coins` (+ (`/Game/Blueprints/BlueprintComponents/AC_Player_inventory.Coins` _player_inventory_2) `Selling Price`) _player_inventory_2)
  (`self.f_Update Coin On UI`)
  (`self.f_Update Selling Item On UI`)
  ;[0 0 0] Save Data
  (`/Game/Blueprints/BlueprintComponents/AC_Player_inventory.f_SaveInventoryData` (`/Game/Blueprints/CharacterBP/BP_ThirdPersonCharacter.Player_inventory` (`self.As BP Third Person Character`))))

(event `IS ShopKeeper On Shop`
  (params (`Show Shop Keeper ?` :type Boolean) (`Can Buy and Sell ?` :type Boolean))
  (`|ExecutionSequence`
    (:`then_0`
      (if `Show Shop Keeper ?`
        (`SkeletalMeshComponent.SetSkeletalMeshAsset` (`self.ShopKeeper`) "/Game/Blueprints/AI_Characters/ShopKeeper/Mesh/ShopKeeper.ShopKeeper")
        (else
          (`SkeletalMeshComponent.SetSkeletalMeshAsset` (`self.ShopKeeper`) null))))
    (:`then_1`
      (if `Can Buy and Sell ?`
        (set `PrimitiveComponent.bGenerateOverlapEvents` true (`self.Box`))
        (else
          (set `PrimitiveComponent.bGenerateOverlapEvents` false (`self.Box`)))))))

(fn `f_Add Items On Inventory`
  (params (`Item Name` :type Name))
  (`KismetArrayLibrary.Array_AddUnique` (`/Game/Blueprints/BlueprintComponents/AC_Player_inventory.Items` (`/Game/Blueprints/CharacterBP/BP_ThirdPersonCharacter.Player_inventory` (`self.As BP Third Person Character`))) `Item Name`))

(fn `f_Add Items Quantity`
  (params (B :type Integer) (Item :type "Name (by ref)"))
  (bind _items_quantity (`/Game/Blueprints/BlueprintComponents/AC_Player_inventory.Items Quantity` (`/Game/Blueprints/CharacterBP/BP_ThirdPersonCharacter.Player_inventory` (`self.As BP Third Person Character`))))
  (`BlueprintMapLibrary.Map_Add` _items_quantity Item (+ (`BlueprintMapLibrary.Map_Find` _items_quantity Item) B)))

(fn `f_Clear All Shop Items`
  (`PanelWidget.ClearChildren` (`/Game/Blueprints/Shop/WB_Shop_System.WrapBox_Shop` (`self.Shop UI`))))

(fn `f_Update Coin On UI`
  (set `/Game/Blueprints/Shop/WB_Shop_System.Coins` (`/Game/Blueprints/BlueprintComponents/AC_Player_inventory.Coins` (`/Game/Blueprints/CharacterBP/BP_ThirdPersonCharacter.Player_inventory` (`self.As BP Third Person Character`))) (`self.Shop UI`)))

(fn `f_Update Items On Shop`
  (for _array_element (`self.Shop Item Static`)
    (bind _returnvalue (`|GetDataTableRow` "/Game/Blueprints/Inventory/Inventory_DataTable.Inventory_DataTable" _array_element)
      (:`then`
        (bind _returnvalue_2 (`|CreateWidget` "/Game/Blueprints/Shop/Item_Buy.Item_Buy_C" null (`.ItemImage_5_F72121984F383ECEA569CE900FBDB1AD` (break `/Game/Blueprints/Inventory/Inventory_Struct` _returnvalue)) (`.BuyingPrice_21_38A785044F0430E961DF84BE3405358B` (break `/Game/Blueprints/Inventory/Inventory_Struct` _returnvalue)) "NewEnumerator0" (break `/Game/Blueprints/Inventory/Inventory_Struct` _returnvalue) self (`.ItemStoreQuantity_17_ABC13BC7442B31160D9701AFB249BFE9` (break `/Game/Blueprints/Inventory/Inventory_Struct` _returnvalue))))
        (`WrapBox.AddChildToWrapBox` (`/Game/Blueprints/Shop/WB_Shop_System.WrapBox_Shop` (`self.Shop UI`)) _returnvalue_2))))
  (for _array_element_2 (`self.Shop Items`)
    (if (not (`KismetArrayLibrary.Array_Contains` (`/Game/Blueprints/BlueprintComponents/AC_Player_inventory.Items` (`/Game/Blueprints/CharacterBP/BP_ThirdPersonCharacter.Player_inventory` (`self.As BP Third Person Character`))) _array_element_2))
      (bind _returnvalue_3 (`|GetDataTableRow` "/Game/Blueprints/Inventory/Inventory_DataTable.Inventory_DataTable" _array_element_2)
        (:`then`
          (bind _returnvalue_4 (`|CreateWidget` "/Game/Blueprints/Shop/Item_Buy.Item_Buy_C" null (`.ItemImage_5_F72121984F383ECEA569CE900FBDB1AD` (break `/Game/Blueprints/Inventory/Inventory_Struct` _returnvalue_3)) (`.BuyingPrice_21_38A785044F0430E961DF84BE3405358B` (break `/Game/Blueprints/Inventory/Inventory_Struct` _returnvalue_3)) "NewEnumerator0" (break `/Game/Blueprints/Inventory/Inventory_Struct` _returnvalue_3) self (`.ItemStoreQuantity_17_ABC13BC7442B31160D9701AFB249BFE9` (break `/Game/Blueprints/Inventory/Inventory_Struct` _returnvalue_3))))
          (`WrapBox.AddChildToWrapBox` (`/Game/Blueprints/Shop/WB_Shop_System.WrapBox_Shop` (`self.Shop UI`)) _returnvalue_4))))))

(fn `f_Update Selling Item On UI`
  (bind _player_inventory (`/Game/Blueprints/CharacterBP/BP_ThirdPersonCharacter.Player_inventory` (`self.As BP Third Person Character`)))
  (`PanelWidget.ClearChildren` (`/Game/Blueprints/Shop/WB_Shop_System.WrapBox_Sell` (`self.Shop UI`)))
  (for _array_element (`/Game/Blueprints/BlueprintComponents/AC_Player_inventory.Items` _player_inventory)
    (bind _returnvalue (`|GetDataTableRow` "/Game/Blueprints/Inventory/Inventory_DataTable.Inventory_DataTable" _array_element)
      (:`then`
        (if (`.CanSellOnShop?_20_1340DA5C41697375FF68B99C56E036A0` (break `/Game/Blueprints/Inventory/Inventory_Struct` _returnvalue))
          (bind _returnvalue_2 (`|CreateWidget` "/Game/Blueprints/Shop/Item_Sell.Item_Sell_C" null (`.ItemImage_5_F72121984F383ECEA569CE900FBDB1AD` (break `/Game/Blueprints/Inventory/Inventory_Struct` _returnvalue)) (`.SellingPrice_25_1F773ABA428E0208CD6C638BA9A906C4` (break `/Game/Blueprints/Inventory/Inventory_Struct` _returnvalue)) (break `/Game/Blueprints/Inventory/Inventory_Struct` _returnvalue) (`BlueprintMapLibrary.Map_Find` (`/Game/Blueprints/BlueprintComponents/AC_Player_inventory.Items Quantity` _player_inventory) _array_element) self))
          (`WrapBox.AddChildToWrapBox` (`/Game/Blueprints/Shop/WB_Shop_System.WrapBox_Sell` (`self.Shop UI`)) _returnvalue_2))))))

(fn `UserConstructionScript`)