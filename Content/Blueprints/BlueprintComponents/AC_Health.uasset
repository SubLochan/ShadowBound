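; Health component for the third-person player character that handles damage, healing, death and UI updates.
; TakeDamage subtracts HP through a DoOnce-plus-delay cooldown macro, and TouchAddHP restores full HP while alive.
; A hit arriving with HP already depleted calls PlayDeath, then reloads the current level after a delay.
; PlayDeath ragdolls the mesh and blocks touch input, except at exactly zero HP, where it only plays a hurt sound.
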(event `Take Damage`
  (params (Damage :type "Float (single-precision)") (DamageType :type "DamageType Object Reference") (InstigatedBy :type "Controller Object Reference") (DamageCauser :type "Actor Object Reference"))
  (bind _hp (`self.HP`))
  ;[0.1256 1 0 1 24] Health System
  (if (and (> _hp 0.0) (!= _hp 0.0))
    (`|ExecutionSequence`
      (:`then_0`
        (`/Engine/EditorBlueprintResources/StandardMacros.DoOnce` false :!label _label
          (:`Completed`
            (set `self.HP` (- (`self.HP`) Damage))
            (`self.Update HP On UI`))))
      (:`then_1`
        (`KismetSystemLibrary.Delay` 0.2)
        (goto _label :!via `Reset`)))
    (else
      (`self.Play Death`)
      (`KismetSystemLibrary.Delay` 5.0)
      (bind _returnvalue (`GameplayStatics.GetCurrentLevelName` true))
      (`GameplayStatics.OpenLevel` (`KismetStringLibrary.Conv_StringToName` _returnvalue)))))

(event `/Game/Blueprints/BlueprintInterface/IF_TouchInterface.Touch Add HP`
  ;[0.1256 1 0 1 24] Health System
  (if (`self.Is Alive?`)
    (set `self.HP` 100.0)
    (`self.Update HP On UI`)))

(event `self.ReceiveTick`
  (params (DeltaSeconds :type "Float (single-precision)")))

(event `self.ReceiveBeginPlay`
  (bind _asbp_third_person_character (cast `/Game/Blueprints/CharacterBP/BP_ThirdPersonCharacter` (`self.GetOwner`)))
  (set `self.Player_ref` _asbp_third_person_character))

(fn `Is Player Alive?`
  (returns (`Is Alive ?` :type Boolean))
  (return false))

(fn `Play Death`
  (bind _player_ref (`self.Player_ref`))
  (if (== (`self.HP`) 0.0)
    (`GameplayStatics.PlaySoundAtLocation` "/Game/SFX/Dammeage/male_hurt7-48124.male_hurt7-48124" (`Actor.K2_GetActorLocation` (`self.Player_ref`)) (struct) 1.0 1.0 0.0 null null null null)
    (else
      (set `self.Is Alive?` false)
      (`CharacterMovementComponent.SetMovementMode` (`Character.CharacterMovement` _player_ref) "MOVE_None" 0)
      (`PrimitiveComponent.SetCollisionEnabled` (`Character.CapsuleComponent` _player_ref) "NoCollision")
      (`PrimitiveComponent.SetSimulatePhysics` (`Character.Mesh` _player_ref) true)
      (`/Game/Blueprints/UI/WBP_UI.Block Touch Input After Player Death` (`/Game/Blueprints/CharacterBP/BP_ThirdPersonCharacter.Main UI` (`self.Player_ref`)))
      (`GameplayStatics.PlaySoundAtLocation` "/Game/SFX/Dammeage/male-death-sound-128357.male-death-sound-128357" (`Actor.K2_GetActorLocation` (`self.Player_ref`)) (struct) 1.0 1.0 0.0 null null null null))))

(fn `Update HP On UI`
  (`/Game/Blueprints/UI/WBP_UI.Update HP On UI` (`/Game/Blueprints/CharacterBP/BP_ThirdPersonCharacter.Main UI` (`self.Player_ref`)) (`self.HP`)))