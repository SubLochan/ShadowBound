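; Player inventory component that holds item names, quantities and coins, loading them from the "Items" save slot on BeginPlay and saving through FSaveInventoryData.
; Middle mouse toggles the inventory widget, filled with item widgets built from Inventory_DataTable rows.
; Clicks route by category: eatables reduce quantity or leave the list and refresh the UI.
; Weapons put their mesh on the character's back, clear the hand mesh and start free-hand mode.
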(event `self.ReceiveBeginPlay`
  (bind _returnvalue (`GameplayStatics.DoesSaveGameExist` "Items"))
  (if _returnvalue
    (bind _returnvalue_2 (`GameplayStatics.LoadGameFromSlot` "Items"))
    (bind _asbp_save_game (cast `/Game/Blueprints/GameSaveSystem/BP_SaveGame` _returnvalue_2))
    (set `self.Items` (`/Game/Blueprints/GameSaveSystem/BP_SaveGame.Items` _asbp_save_game))
    (set `self.Items Quantity` (`/Game/Blueprints/GameSaveSystem/BP_SaveGame.Items Quantity` _asbp_save_game))
    (set `self.Coins` (`/Game/Blueprints/GameSaveSystem/BP_SaveGame.Coins` _asbp_save_game))))

(event `Update Inventory`
  (if (`self.Inventory Open ?`)
    (`PanelWidget.ClearChildren` (`/Game/Blueprints/Inventory/WBP_Inventory.WrapBoxInventory` (`self.UI Inventroy`)))
    (for _array_element (`self.Items`) :!label _label
      (bind _returnvalue (`|GetDataTableRow` "/Game/Blueprints/Inventory/Inventory_DataTable.Inventory_DataTable" _array_element)
        (:`then`
          (bind (_itemname _itemimage _itemcategory) (break `/Game/Blueprints/Inventory/Inventory_Struct` _returnvalue))
          (bind _returnvalue_2 (`|CreateWidget` "/Game/Blueprints/Inventory/Item_Inventory.Item_Inventory_C" null _itemimage (`BlueprintMapLibrary.Map_Find` (`self.Items Quantity`) _array_element) _itemcategory _itemname self))
          (`WrapBox.AddChildToWrapBox` (`/Game/Blueprints/Inventory/WBP_Inventory.WrapBoxInventory` (`self.UI Inventroy`)) _returnvalue_2))))))

(event `Open Inventory On Component`
  (bind _returnvalue (`|CreateWidget` "/Game/Blueprints/Inventory/WBP_Inventory.WBP_Inventory_C" null (`self.Coins`) :!label _label_2))
  (bind _output_get (set `self.UI Inventroy` _returnvalue))
  (`UserWidget.AddToViewport` _output_get 0)
  (goto _label))

(event `Key|MiddleMouseButton`
  (params (Key :type "Key Structure"))
  (:`Pressed`
    (`/Engine/EditorBlueprintResources/StandardMacros.FlipFlop`
      (:`A`
        (set `self.Inventory Open ?` true)
        (goto _label_2))
      (:`B`
        (set `self.Inventory Open ?` false)
        (`Widget.RemoveFromParent` (`self.UI Inventroy`))))))

(event `On Click Item`
  (params (Category :type "/Game/Blueprints/Inventory/E_Item_Category Enum" :default "NewEnumerator0") (`Item Name` :type String) (`Item Quantity` :type Integer))
  (bind _returnvalue (`KismetStringLibrary.Conv_StringToName` `Item Name`))
  (bind _items_quantity (`self.Items Quantity`))
  (bind _value (`BlueprintMapLibrary.Map_Find` _items_quantity _returnvalue))
  (switch `/Game/Blueprints/Inventory/E_Item_Category` Category
    (:`NewEnumerator1`
      (if (> _value 1)
        (`BlueprintMapLibrary.Map_Add` _items_quantity _returnvalue (- _value `Item Quantity`))
        (`self.Update Inventory`)
        (else
          (`KismetArrayLibrary.Array_RemoveItem` (`self.Items`) _returnvalue)
          (`BlueprintMapLibrary.Map_Add` (`self.Items Quantity`))
          (`self.Update Inventory`))))
    (:`NewEnumerator2`
      (bind _asbp_third_person_character (cast `/Game/Blueprints/CharacterBP/BP_ThirdPersonCharacter` (`self.GetOwner`)))
      (bind _returnvalue_2 (`|GetDataTableRow` "/Game/Blueprints/Inventory/Inventory_DataTable.Inventory_DataTable" (`KismetStringLibrary.Conv_StringToName` `Item Name`))
        (:`then`
          (bind _output_get (set `/Game/Blueprints/CharacterBP/BP_ThirdPersonCharacter.Weapon` (`.StaticMesh_11_B51CCB664DC8BE69913D47B61BA8D2CB` (break `/Game/Blueprints/Inventory/Inventory_Struct` _returnvalue_2)) _asbp_third_person_character))
          (`StaticMeshComponent.SetStaticMesh` (`/Game/Blueprints/CharacterBP/BP_ThirdPersonCharacter.Weapon On Hand` _asbp_third_person_character) null)
          (`StaticMeshComponent.SetStaticMesh` (`/Game/Blueprints/CharacterBP/BP_ThirdPersonCharacter.WeaponOnBack` _asbp_third_person_character) _output_get)
          (`/Game/Blueprints/CharacterBP/BP_ThirdPersonCharacter.f_Start Free Hand Mode` _asbp_third_person_character))))))

(fn `f_SaveInventoryData`
  (bind _returnvalue (`GameplayStatics.CreateSaveGameObject` "/Game/Blueprints/GameSaveSystem/BP_SaveGame.BP_SaveGame_C"))
  (set `/Game/Blueprints/GameSaveSystem/BP_SaveGame.Items` (`self.Items`) _returnvalue)
  (set `/Game/Blueprints/GameSaveSystem/BP_SaveGame.Items Quantity` (`self.Items Quantity`) _returnvalue)
  (set `/Game/Blueprints/GameSaveSystem/BP_SaveGame.Coins` (`self.Coins`) _returnvalue)
  (`GameplayStatics.SaveGameToSlot` _returnvalue "Items")
  (`KismetSystemLibrary.PrintString` "Save Game - Items"))